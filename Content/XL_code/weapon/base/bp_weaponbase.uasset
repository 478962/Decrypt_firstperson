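; Base weapon Blueprint for automatic hitscan fire, driven by a looping timer from StartWeaponFire until stopfire.
; Each shot plays weapon and arm montages chosen by player state, spawns muzzle flash and casing, and kicks the camera for recoil.
; A camera-forward line trace switches on physical surface type to spawn impact effects, sounds and decals, without applying damage.
; Ammo is checked only when firing starts and is never decremented here.
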(event `fire internal`
  (bind _player (`self.Player`))
  (bind (_returnvalue_location _returnvalue_rotation) (`KismetMathLibrary.BreakTransform` (`SceneComponent.GetSocketTransform` (`self.weapon`) "casing" "RTS_World")))
  (bind _camera (`/Game/XL_code/player/bp_FpsPlayer.Camera` (`self.Player`)))
  (bind _returnvalue (`SceneComponent.K2_GetComponentLocation` _camera))
  (`|PlayMontage` (`self.weapon`) (select `/Game/XL_code/player/enum/E_playerState` (`/Game/XL_code/player/bp_FpsPlayer.E_playerState` (`self.Player`)) :`NewEnumerator0` (`self.weapon Idle`) :`NewEnumerator1` (`self.weapon Walk`) :`NewEnumerator3` (`self.weapon Aim`))
    (:`then`
      (`|PlayMontage` (`/Game/XL_code/player/bp_FpsPlayer.arm` (`self.Player`)) (select `/Game/XL_code/player/enum/E_playerState` (`/Game/XL_code/player/bp_FpsPlayer.E_playerState` (`self.Player`)) :`NewEnumerator0` (`self.player Idle`) :`NewEnumerator1` (`self.player Walk`) :`NewEnumerator3` (`self.player Aim`))
        (:`then`
          (`GameplayStatics.PlaySound2D` "/Game/XL_code/weapon/MetaSound/Ms_virtus.Ms_virtus" 1.0 1.0 0.0 null null)
          (`NiagaraFunctionLibrary.SpawnSystemAttached` "/Game/ShotSystem/Shot_VFX/VIRTUS_MuzzleFlash.VIRTUS_MuzzleFlash" (`self.barrel`) "Muzzle" (0.0 0.0 0.0) (struct) "KeepRelativeOffset" true)
          (`|SpawnActorFromClass` "/Game/XL_code/weapon/bp_casing.bp_casing_C" (`KismetMathLibrary.MakeTransform` _returnvalue_location _returnvalue_rotation) "Undefined" "MultiplyWithRoot" null null)
          (`Pawn.AddControllerPitchInput` _player -0.4)
          (`Pawn.AddControllerYawInput` _player (`KismetMathLibrary.RandomFloatInRange` -0.1 0.1))
          (bind _outhit (`KismetSystemLibrary.LineTraceSingle` _returnvalue (+ _returnvalue (* (`SceneComponent.GetForwardVector` _camera) 10000)) "TraceTypeQuery1"))
          (bind (_bblockinghit _binitialoverlap _time _distance _location _impactpoint _normal _impactnormal _physmat) (`GameplayStatics.BreakHitResult` _outhit))
          (if _bblockinghit
            (set `self.Location` _location)
            (switch `EPhysicalSurface` (`PhysicalMaterial.SurfaceType` _physmat)
              (:`SurfaceType_Default`
                (bind _returnvalue_2 (`KismetMathLibrary.MakeRotFromX` _normal))
                (`NiagaraFunctionLibrary.SpawnSystemAtLocation` "/Game/ShotSystem/Shot_VFX/FX_SquibConcrete.FX_SquibConcrete" (`self.Location`) _returnvalue_2 :!label _label)
                (`GameplayStatics.SpawnSoundAtLocation` "/Game/XL_FPSPack/Common/Sound/Bullet_Impact_Sounds/Concrete/Hit_Concrete.Hit_Concrete" (`self.Location`) (struct) 0.5 1.0 0.0 null null)
                (`|SpawnActorFromClass` "/Game/Decals/BP_BulletDecal.BP_BulletDecal_C" (`KismetMathLibrary.MakeTransform` (`self.Location`) _returnvalue_2 (0.4 0.4 0.4)) "Undefined" "MultiplyWithRoot" null null))
              (:`SurfaceType1`
                (`NiagaraFunctionLibrary.SpawnSystemAtLocation` "/Game/ShotSystem/Shot_VFX/FX_SquibDirt.FX_SquibDirt" (`self.Location`) _returnvalue_2)
                (`GameplayStatics.SpawnSoundAtLocation` "/Game/ShotSystem/Shot_SFX/SFX_Vefects_Shots_Squib_Dirt_Cue.SFX_Vefects_Shots_Squib_Dirt_Cue" (`self.Location`) (struct) 1.0 1.0 0.0 null null)
                (`|SpawnActorFromClass` "/Game/Decals/BP_BulletDecal.BP_BulletDecal_C" (`KismetMathLibrary.MakeTransform` (`self.Location`) _returnvalue_2 (0.4 0.4 0.4)) "Undefined" "MultiplyWithRoot" null null))
              (:`SurfaceType2`
                (`NiagaraFunctionLibrary.SpawnSystemAtLocation` "/Game/ShotSystem/Shot_VFX/FX_SquibMetal.FX_SquibMetal" (`self.Location`) _returnvalue_2)
                (`GameplayStatics.SpawnSoundAtLocation` "/Game/ShotSystem/Shot_SFX/SFX_Vefects_Shots_Squib_Metal_Cue.SFX_Vefects_Shots_Squib_Metal_Cue" (`self.Location`) (struct) 2.0 1.0 0.0 null null)
                (bind _returnvalue_3 (`|SpawnActorFromClass` "/Game/Decals/BP_BulletDecal.BP_BulletDecal_C" (`KismetMathLibrary.MakeTransform` (`self.Location`) _returnvalue_2 (0.4 0.4 0.4)) "Undefined" "MultiplyWithRoot" null null))
                (`DecalComponent.SetDecalMaterial` (`/Game/Decals/BP_BulletDecal.BulletDecal` _returnvalue_3) "/Game/Decals/Materials/MI_VFX_BulletDecal_Metal.MI_VFX_BulletDecal_Metal"))
              (:`SurfaceType3`
                (`NiagaraFunctionLibrary.SpawnSystemAtLocation` "/Game/ShotSystem/Shot_VFX/FX_SquibWood.FX_SquibWood" (`self.Location`) _returnvalue_2)
                (`GameplayStatics.SpawnSoundAtLocation` "/Game/ShotSystem/Shot_SFX/SFX_Vefects_Shots_Squib_Wood_Cue.SFX_Vefects_Shots_Squib_Wood_Cue" (`self.Location`) (struct) 1.0 1.0 0.0 null null)
                (bind _returnvalue_4 (`|SpawnActorFromClass` "/Game/Decals/BP_BulletDecal.BP_BulletDecal_C" (`KismetMathLibrary.MakeTransform` (`self.Location`) _returnvalue_2 (0.4 0.4 0.4)) "Undefined" "MultiplyWithRoot" null null))
                (`DecalComponent.SetDecalMaterial` (`/Game/Decals/BP_BulletDecal.BulletDecal` _returnvalue_4) "/Game/Decals/Materials/MI_VFX_BulletDecal_Wood.MI_VFX_BulletDecal_Wood"))
              (:`SurfaceType4`
                (`NiagaraFunctionLibrary.SpawnSystemAtLocation` "/Game/XL_FPSPack/Niagara_VFX/Niagara/Impact/Impact_Blood.Impact_Blood" (`self.Location`) _returnvalue_2)
                (`GameplayStatics.SpawnSoundAtLocation` "/Game/XL_FPSPack/Common/Sound/Bullet_Impact_Sounds/Concrete/Hit_Concrete.Hit_Concrete" (`self.Location`) (struct) 1.0 1.0 0.0 null null)
                (`|SpawnActorFromClass` "/Game/Decals/BP_BulletDecal.BP_BulletDecal_C" (`KismetMathLibrary.MakeTransform` (`self.Location`) _returnvalue_2 (0.4 0.4 0.4)) "Undefined" "MultiplyWithRoot" null null))
              (:`SurfaceType5`
                (goto _label)))))))))

(event `/Game/XL_blueprintInterface/BI_fire.start weapon fire`
  (params (player :type "/Game/XL_code/player/bp_FpsPlayer Object Reference"))
  (set `self.Player` player)
  (if (> (`self.current ammo`) 0)
    (`self.fire internal`)
    (bind _returnvalue (`KismetSystemLibrary.K2_SetTimerDelegate` (delegate `fire internal`) (`self.fire rate`) true))
    (set `self.fire timer handle` _returnvalue)))

(event `stop fire`
  (`KismetSystemLibrary.K2_ClearAndInvalidateTimerHandle` (`self.fire timer handle`)))

(fn `GetAimSocketLocation`
  (returns (AimSocketLocation :type "Vector Structure"))
  (bind _output_get (set `self.AimSocketLocation` (`SceneComponent.GetSocketLocation` (`self.weapon`) "aimsocket")))
  (return _output_get))

(fn `UserConstructionScript`)